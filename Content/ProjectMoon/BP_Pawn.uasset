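; VR player pawn with smooth camera-relative movement, snap turning and jump through Enhanced Input.
; On BeginPlay it adds the mapping context, offsets VRRoot to the desired camera height after a delay, and spawns two BP_Hand actors attached to VRRoot.
; Snap turns rotate the actor, then offset it so the camera stays in place.
; Tick feeds head and hand transforms to the mannequin AnimBlueprint to drive the body.
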(event `self.ReceiveBeginPlay`
  (bind (_returnvalue_x _returnvalue_y _returnvalue_z) (`KismetMathLibrary.BreakVector` (`SceneComponent.K2_GetComponentLocation` (`self.Camera`))))
  (`|ExecutionSequence`
    (:`then_0`
      (`EnhancedInputSubsystemInterface.AddMappingContext` (pcsubsystem `EnhancedInputLocalPlayerSubsystem` (`GameplayStatics.GetPlayerController` 0)) "/Game/ProjectMoon/Move/VRMoveTest.VRMoveTest" 0 (struct)))
    (:`then_1`
      (`HeadMountedDisplayFunctionLibrary.SetTrackingOrigin` "Stage")
      (`KismetSystemLibrary.Delay` 1.0)
      (`SceneComponent.K2_AddRelativeLocation` (`self.VRRoot`) (`KismetMathLibrary.MakeVector` 0.0 0.0 (- (`self.DesiredCameraHeight`) _returnvalue_z)) false false))
    (:`then_2`
      (bind _returnvalue (`|SpawnActorFromClass` "/Game/ProjectMoon/BP_Hand.BP_Hand_C" (`KismetMathLibrary.MakeTransform` (0.0 0.0 0.0)) "AlwaysSpawn" "MultiplyWithRoot" self true null))
      (bind _output_get (set `self.LeftHand` _returnvalue))
      (`self.K2_AttachToComponent` _output_get (`self.VRRoot`) "None" "SnapToTarget" "SnapToTarget" "KeepRelative" true))
    (:`then_3`
      (bind _returnvalue_2 (`|SpawnActorFromClass` "/Game/ProjectMoon/BP_Hand.BP_Hand_C" (`KismetMathLibrary.MakeTransform` (0.0 0.0 0.0)) "AlwaysSpawn" "MultiplyWithRoot" self false null))
      (bind _output_get_2 (set `self.RightHand` _returnvalue_2))
      (`self.K2_AttachToComponent` _output_get_2 (`self.VRRoot`) "None" "SnapToTarget" "SnapToTarget" "KeepRelative" true))))

(event `EnhancedInput|/Game/ProjectMoon/Move/VRMove`
  (params (ActionValue :type "Float (double-precision)") (ElapsedSeconds :type "Float (double-precision)") (TriggeredSeconds :type "Float (double-precision)") (InputAction :type "InputAction Object Reference" :default "/Game/ProjectMoon/Move/VRMove.VRMove"))
  (bind (_returnvalue_x _returnvalue_y) (`KismetMathLibrary.BreakVector` (`SceneComponent.GetForwardVector` (`self.Camera`))))
  (:`Triggered`
    (`self.AddMovementInput` (`KismetMathLibrary.MakeVector` _returnvalue_x _returnvalue_y) ActionValue)))

(event `EnhancedInput|/Game/ProjectMoon/Move/VRTurn`
  (params (ActionValue :type "Float (double-precision)") (ElapsedSeconds :type "Float (double-precision)") (TriggeredSeconds :type "Float (double-precision)") (InputAction :type "InputAction Object Reference" :default "/Game/ProjectMoon/Move/VRTurn.VRTurn"))
  (:`Triggered`
    (`self.Snap turn` (> ActionValue 0.0))))

(event `EnhancedInput|/Game/ProjectMoon/Move/VRJump`
  (params (ActionValue :type Boolean) (ElapsedSeconds :type "Float (double-precision)") (TriggeredSeconds :type "Float (double-precision)") (InputAction :type "InputAction Object Reference" :default "/Game/ProjectMoon/Move/VRJump.VRJump"))
  (:`Triggered`
    (`Character.Jump` (`GameplayStatics.GetPlayerCharacter` 0))))

(event `self.ReceiveTick`
  (params (DeltaSeconds :type "Float (single-precision)"))
  (bind _assk_mannequin_anim_blueprint (cast `/Game/ControlRig/Characters/Mannequins/Meshes/SK_Mannequin_AnimBlueprint` (`SkeletalMeshComponent.GetAnimInstance` (`self.SkeletalMesh`))))
  (set `/Game/ControlRig/Characters/Mannequins/Meshes/SK_Mannequin_AnimBlueprint.HeadTransform` (`SceneComponent.K2_GetComponentToWorld` (`self.Camera`)) _assk_mannequin_anim_blueprint)
  (set `/Game/ControlRig/Characters/Mannequins/Meshes/SK_Mannequin_AnimBlueprint.LeftHandTransform` (`SceneComponent.K2_GetComponentToWorld` (`Actor.RootComponent` (`self.LeftHand`))) _assk_mannequin_anim_blueprint)
  (set `/Game/ControlRig/Characters/Mannequins/Meshes/SK_Mannequin_AnimBlueprint.RightHandTransform` (`SceneComponent.K2_GetComponentToWorld` (`Actor.RootComponent` (`self.RightHand`))) _assk_mannequin_anim_blueprint))

(fn `Snap turn`
  (params (bRightTurn :type Boolean))
  (locals (LocalPrevCameraLocation :type "Vector Structure") (LocalYawDelta :type "Float (double-precision)"))
  (bind _snapturndegrees (`self.SnapTurnDegrees`))
  (set `local.LocalPrevCameraLocation` (`SceneComponent.K2_GetComponentLocation` (`self.Camera`)))
  (`self.K2_AddActorWorldRotation` (`KismetMathLibrary.MakeRotator` 0.0 0.0 (`KismetMathLibrary.SelectFloat` (`KismetMathLibrary.Abs` _snapturndegrees) _snapturndegrees (`local.bRightTurn`))) false true)
  (`self.K2_AddActorWorldOffset` (- (`local.LocalPrevCameraLocation`) (`SceneComponent.K2_GetComponentLocation` (`self.Camera`)))))

(fn `UserConstructionScript`)