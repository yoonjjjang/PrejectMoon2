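; BP_Hand is a VR hand actor that serves as either the left or right hand, depending on the LeftHand flag.
; On BeginPlay it assigns the matching MannyXR hand mesh, rotates it for that side and sets the MotionController's motion source to Left or Right.
; Overlap, Tick and the construction script are empty, so all logic is this one-time setup.
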(event `self.ReceiveBeginPlay`
  (if (`self.bLeftHand`)
    (`SkeletalMeshComponent.SetSkeletalMeshAsset` (`self.HandMesh`) "/Game/Characters/MannequinsXR/Meshes/SKM_MannyXR_left.SKM_MannyXR_left")
    (`SceneComponent.K2_SetRelativeRotation` (`self.HandMesh`) (struct :`Pitch` -90.0 :`Roll` -90.0) false false)
    (set `MotionControllerComponent.MotionSource` "Left" (`self.MotionController`))
    (else
      (`SkeletalMeshComponent.SetSkeletalMeshAsset` (`self.HandMesh`) "/Game/Characters/MannequinsXR/Meshes/SKM_MannyXR_right.SKM_MannyXR_right")
      (`SceneComponent.K2_SetRelativeRotation` (`self.HandMesh`) (struct :`Pitch` 90.0 :`Roll` 90.0) false false)
      (set `MotionControllerComponent.MotionSource` "Right" (`self.MotionController`)))))

(fn `UserConstructionScript`)