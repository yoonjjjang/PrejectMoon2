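; BP_MirroredFullVRBody is an actor that shows a mirrored copy of the player's VR body.
; On BeginPlay it hands the VR pawn's mesh to ABP_MirroredPawn as PlayerSkeleton and scales its own mesh by eye-level height relative to 180.
; Each Tick it copies the player mesh transform with world Y negated and yaw flipped, mirroring across the world Y=0 plane, and prints its location.
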(event `self.ReceiveBeginPlay`
  (bind _asvrpawn (cast `/Game/VRTemplate/Blueprints/VRPawn` (`Controller.K2_GetPawn` (`GameplayStatics.GetPlayerController` 0))))
  (set `self.PlayerSkeletalMesh` (`Character.Mesh` _asvrpawn))
  (bind _asabp_mirrored_pawn (cast `/Game/ABP_MirroredPawn` (`SkeletalMeshComponent.GetAnimInstance` (`self.SkeletalMesh`))))
  (set `/Game/ABP_MirroredPawn.PlayerSkeleton` (`self.PlayerSkeletalMesh`) _asabp_mirrored_pawn)
  (bind (_relativelocation_x _relativelocation_y _relativelocation_z) (`KismetMathLibrary.BreakVector` (`SceneComponent.RelativeLocation` (`/Game/VRTemplate/Blueprints/VRPawn.EyeLevelComponent` _asvrpawn))))
  (`SceneComponent.SetRelativeScale3D` (`self.SkeletalMesh`) (`KismetMathLibrary.Conv_DoubleToVector` (/ _relativelocation_z 180.0))))

(event `self.ReceiveTick`
  (params (DeltaSeconds :type "Float (single-precision)"))
  (bind _returnvalue (`SceneComponent.K2_GetComponentToWorld` (`self.PlayerSkeletalMesh`)))
  (`SceneComponent.K2_SetWorldTransform` (`self.SkeletalMesh`) (`KismetMathLibrary.MakeTransform` (`KismetMathLibrary.MakeVector` (.x (.location _returnvalue)) (* (.y (.location _returnvalue)) -1.0) (.z (.location _returnvalue))) (`KismetMathLibrary.MakeRotator` (.roll (.rotation _returnvalue)) (.pitch (.rotation _returnvalue)) (* (+ (.yaw (.rotation _returnvalue)) 180.0) -1.0))) false false)
  (`KismetSystemLibrary.PrintText` (`KismetTextLibrary.Conv_VectorToText` (`SceneComponent.K2_GetComponentLocation` (`self.SkeletalMesh`)))))

(fn `UserConstructionScript`)